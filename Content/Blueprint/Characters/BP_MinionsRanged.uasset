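; BP_MinionsRanged is a ranged minion character that shoots a given enemy and can itself be killed.
; It sets health to its maximum on BeginPlay, subtracts incoming damage, and destroys itself at zero or below.
; StartShooting plays explosion effects at its Sphere, draws a debug visibility trace to the target, then applies fixed damage regardless of the trace result.
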(event Custom|StartShooting
  (params (EnemyToShoot :type Actor%20Object%20Reference))
  (bind _sphere (Variables|Default|GetSphere))
  (bind _returnvalue (Transformation|GetWorldLocation _sphere))
  (Effects|SpawnEmitteratLocation "/Game/StarterContent/Particles/P_Explosion.P_Explosion" _returnvalue)
  (Audio|PlaySoundatLocation "/Game/StarterContent/Audio/Explosion_Cue.Explosion_Cue" _returnvalue "0, 0, 0" 1.0 1.0 0.0 0 0 0)
  (Collision|LineTraceByChannel (Transformation|GetActorLocation) (Transformation|GetActorLocation EnemyToShoot) "TraceTypeQuery1" false 0 "ForDuration")
  (Game|Damage|ApplyDamage EnemyToShoot 19.0 0 self "/Script/Engine.DamageType"))

(event EventBeginPlay
  (Variables|Default|SetHeath (Variables|Default|GetMaxHealth)))

(event Game|Damage|EventAnyDamage
  (params (Damage :type Float%20%28single-precision%29) (DamageType :type Damage%20Type%20Object%20Reference) (InstigatedBy :type Controller%20Object%20Reference) (DamageCauser :type Actor%20Object%20Reference))
  (bind _output_get (Variables|Default|SetHeath (- (Variables|Default|GetHeath) Damage)))
  (if (<= _output_get 0.0)
    (Actor|DestroyActor)))

(fn ConstructionScript)